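; An AI controller Blueprint for detection behavior, with movement driven by an Idle, Suspicious, Searching or Alert state.
; BeginPlay caches the player character and runs UpdateState once, which switches on CurrentState.
; Suspicious and Searching move toward LastHeardLocation at different acceptance radii, while Alert moves to the player.
; Idle re-calls UpdateState when the player is near, but nothing here changes the state or sets the heard location.
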(event `self.ReceiveBeginPlay`
  (bind _asbp_third_person_character (cast `/Game/ThirdPerson/Blueprints/BP_ThirdPersonCharacter` (`GameplayStatics.GetPlayerPawn` 0)))
  (`self.Update State`))

(event `Update State`
  (switch `EDetectionState` (`self.CurrentState`)
    (:`Idle`
      (`KismetSystemLibrary.PrintString` "w")
      (if (<= (`self.GetDistanceTo` (stale `self.ReceiveBeginPlay` _asbp_third_person_character)) 400.0)
        (`self.Update State`)))
    (:`Suspicious`
      (`self.MoveToLocation` (`self.LastHeardLocation`) 400.0 true true false true null)
      (`KismetSystemLibrary.PrintString` "Hello"))
    (:`Searching`
      (`self.MoveToLocation` (`self.LastHeardLocation`) 100.0 true true false true null))
    (:`Alert`
      (`self.MoveToActor` (`GameplayStatics.GetPlayerCharacter` 0) 149.0 true true true null))))

(fn `UserConstructionScript`)